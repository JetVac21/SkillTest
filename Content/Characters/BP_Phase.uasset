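; BP_Phase is a character Blueprint that handles a projectile ability in three events: spawn, cancel and launch.
; Spawning attaches a BP_Projectile to the mesh's projectile socket and plays the ability intro montage, while cancelling destroys it and stops the montage.
; Launching detaches and shoots the projectile, then plays the montage's Fire section, whose "Fire Projectile" notify calls ShootProjectile again.
; A particle activation call is left unconnected.
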(event `SpawnProjectile`
  (bind _returnvalue (`|SpawnActorFromClass` "/Game/Characters/BP_Projectile.BP_Projectile_C" (`KismetMathLibrary.MakeTransform` (0.0 0.0 0.0)) "Undefined" "MultiplyWithRoot" null null))
  (bind _output_get (set `self.Projectile` _returnvalue))
  (`self.K2_AttachToComponent` _output_get (`self.Mesh`) "projectile_socket" "KeepRelative" "KeepRelative" "KeepWorld" true)
  (`|PlayMontage` (`self.Mesh`) "/Game/Characters/Animations/AM_Ability_Intro.AM_Ability_Intro"))

(event `CancelProjectile`
  (`self.K2_DestroyActor` (`self.Projectile`))
  (`self.StopAnimMontage` "/Game/Characters/Animations/AM_Ability_Intro.AM_Ability_Intro"))

(event `LaunchProjectile`
  (`self.K2_DetachFromActor` (`self.Projectile`) "KeepWorld" "KeepWorld" "KeepWorld")
  (`/Game/Characters/BP_Projectile.ShootProjectile` (`self.Projectile`) self)
  (bind _notifyname (`|PlayMontage` (`self.Mesh`) "/Game/Characters/Animations/AM_Ability_Intro.AM_Ability_Intro" 1.0 0.0 "Fire")
    (:`OnNotifyBegin`
      (if (== _notifyname "Fire Projectile")
        (`/Game/Characters/BP_Projectile.ShootProjectile` (`self.Projectile`) self)))))

(fn `UserConstructionScript`
  (`parent.UserConstructionScript`))